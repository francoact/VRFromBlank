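; BP_PickUpBomb_A is a bomb actor in VRTest that explodes when it is struck hard enough.
; On a component hit, it compares the length of the normal impulse against a minimum detonation force.
; Above that threshold it spawns an explosion particle effect, hides the mesh, stops its physics simulation, and destroys itself after a short delay.
; The explosion is visual only, with no damage or force applied in this graph.
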(event `self.StaticMeshComponent.OnComponentHit`
  (params (HitComponent :type "PrimitiveComponent Object Reference") (OtherActor :type "Actor Object Reference") (OtherComp :type "PrimitiveComponent Object Reference") (NormalImpulse :type "Vector Structure") (Hit :type "HitResult Structure (by ref)"))
  (bind _staticmeshcomponent (`self.StaticMeshComponent`))
  (if (> (`KismetMathLibrary.VSize` NormalImpulse) (`self.MinimalForceToDetonate`))
    (`GameplayStatics.SpawnEmitterAtLocation` "/Game/StarterContent/Particles/P_Explosion.P_Explosion" (`self.K2_GetActorLocation`))
    (`SceneComponent.SetVisibility` _staticmeshcomponent false false)
    (`PrimitiveComponent.SetSimulatePhysics` _staticmeshcomponent false)
    (`KismetSystemLibrary.Delay` 0.5)
    (`self.K2_DestroyActor`)))

(fn `UserConstructionScript`
  (`parent.UserConstructionScript`))