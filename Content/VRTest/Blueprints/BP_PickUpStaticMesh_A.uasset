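; BP_PickUpStaticMesh_A is a VR test static mesh actor that can be picked up and dropped.
; Pickup turns off physics simulation and attaches the mesh to the given component, either snapping location and rotation or keeping world transform based on SnapOnPickup.
; Drop re-enables physics and detaches the mesh in place, with both events updating the IsPickedUp flag.
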(event `/Game/VRFeature/VirtualRealityBP/Blueprints/PickupActorInterface.Pickup`
  (params (AttachTo :type "SceneComponent Object Reference"))
  (bind _returnvalue (select `bool` (`self.SnapOnPickup`) :`false` "KeepWorld" :`true` "SnapToTarget" :!type "EAttachmentRule Enum"))
  (`PrimitiveComponent.SetSimulatePhysics` (`self.StaticMeshComponent`) false)
  (`SceneComponent.K2_AttachToComponent` (`self.StaticMeshComponent`) AttachTo "None" _returnvalue _returnvalue "KeepWorld" false)
  (set `self.IsPickedUp` true))

(event `/Game/VRFeature/VirtualRealityBP/Blueprints/PickupActorInterface.Drop`
  (`PrimitiveComponent.SetSimulatePhysics` (`self.StaticMeshComponent`) true)
  (`SceneComponent.K2_DetachFromComponent` (`self.StaticMeshComponent`) "KeepWorld" "KeepWorld" "KeepWorld" true)
  (set `self.IsPickedUp` false))

(fn `UserConstructionScript`)