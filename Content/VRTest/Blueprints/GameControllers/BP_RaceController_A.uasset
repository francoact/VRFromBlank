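; BP_RaceController_A runs a timed race by linking a movable object, a mark collection and a chronometer through event bindings.
; Movement start restarts the chronometer, and the collection's finish condition stops it, saves the time under a numbered "Jugador" name, then resets marks and position after a delay.
; The collection's reset condition resets both immediately.
; Scores persist in a BP_RaceData_SG save game, loaded and printed on BeginPlay.
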(event `self.ReceiveBeginPlay`
  (`self.LoadRaceData`))

(event `self.RefMovilObject.MoveStarted`
  (`self.StartRace`))

(event `self.RefMarkCollection.FinishConditionReached`
  (`self.EndRace`)
  (`KismetSystemLibrary.Delay` 5.0)
  (`/Game/VRTest/Blueprints/Mechanisms/BP_MarkCollection_A.ResetCollection` (`self.RefMarkCollection`))
  (`/Game/VRTest/Blueprints/Mechanisms/BP_MovilObject_A.RestartPosition` (`self.RefMovilObject`)))

(event `self.RefMarkCollection.ResetConditionReached`
  (`/Game/VRTest/Blueprints/Mechanisms/BP_MarkCollection_A.ResetCollection` (`self.RefMarkCollection`))
  (`/Game/VRTest/Blueprints/Mechanisms/BP_MovilObject_A.RestartPosition` (`self.RefMovilObject`)))

(fn `EndRace`
  (bind _refchronometer (`self.RefChronometer`))
  (bind _racedata (`self.RaceData`))
  (`/Game/VRTest/Blueprints/Mechanisms/BP_Chronometer_A.Stop` _refchronometer)
  (`/Game/VRTest/Blueprints/GameControllers/BP_RaceData_SG.AddScoreRegistry` _racedata (`KismetStringLibrary.Concat_StrStr` "Jugador " (`KismetStringLibrary.Conv_IntToString` (`BlueprintMapLibrary.Map_Length` (`/Game/VRTest/Blueprints/GameControllers/BP_RaceData_SG.ScoreList` _racedata)))) (`/Game/VRTest/Blueprints/Mechanisms/BP_Chronometer_A.Time` _refchronometer))
  (`/Game/VRTest/Blueprints/GameControllers/BP_RaceData_SG.SaveData` _racedata))

(fn `LoadRaceData`
  (`|ExecutionSequence`
    (:`then_0`
      (bind _returnvalue (`GameplayStatics.CreateSaveGameObject` "/Game/VRTest/Blueprints/GameControllers/BP_RaceData_SG.BP_RaceData_SG_C"))
      (bind _output_get (set `self.RaceData` _returnvalue))
      (bind _returnvalue_2 (`GameplayStatics.LoadGameFromSlot` (`/Game/VRTest/Blueprints/GameControllers/BP_RaceData_SG.SlotName` _output_get)))
      (bind _asbp_race_data_sg (cast `/Game/VRTest/Blueprints/GameControllers/BP_RaceData_SG` _returnvalue_2))
      (set `self.RaceData` _asbp_race_data_sg))
    (:`then_1`
      (`/Game/VRTest/Blueprints/GameControllers/BP_RaceData_SG.PrintData` (`self.RaceData`)))))

(fn `StartRace`
  (`/Game/VRTest/Blueprints/Mechanisms/BP_Chronometer_A.Reset` (`self.RefChronometer`))
  (`/Game/VRTest/Blueprints/Mechanisms/BP_Chronometer_A.Start` (`self.RefChronometer`)))

(fn `UserConstructionScript`)