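; BP_RaceData_SG is a SaveGame object that stores race scores in a ScoreList map of names to points.
; AddScoreRegistry adds an entry to the map, and SaveData writes the object itself to its SlotName save slot.
; PrintData is currently empty, as its debug loop that prints each name and score is left disconnected.
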(fn `AddScoreRegistry`
  (params (Name :type String) (Poins :type "Float (double-precision)"))
  (`BlueprintMapLibrary.Map_Add` (`self.ScoreList`) Name Poins))

(fn `PrintData`)

(fn `SaveData`
  (`GameplayStatics.SaveGameToSlot` self (`self.SlotName`)))