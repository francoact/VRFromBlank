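; VR pickup gun that, while held, shows an ammo counter widget and a laser mark on enemies in its line of fire.
; Firing spawns a projectile from the Arrow, rumbles the holding controller, plays audio and updates the counter.
; A magazine overlapping the collision box binds to its drop event; dropping it there copies its ammo into the gun and destroys it.
; A per-tick line trace positions the laser billboard just short of the enemy hit.
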(event `/Game/VRFeature/VirtualRealityBP/Blueprints/PickupActorInterface.Pickup`
  (params (AttachTo :type "SceneComponent Object Reference"))
  (`parent.Pickup` AttachTo)
  ;[1 1 1] Guardar MotionController
  (bind _asbp_motion_controller_a (cast `/Game/VRTest/Blueprints/BP_MotionController_A` (`ActorComponent.GetOwner` AttachTo)))
  (set `self.Ref_CurrentController` _asbp_motion_controller_a)
  ;[1 1 1] Reubicar arma
  (`self.K2_AddActorLocalRotation` self (struct :`Yaw` -90.0) false false)
  (`self.K2_AddActorLocalOffset` self (0.0 -6.0 -3.0) false false)
  (`SceneComponent.SetVisibility` (`self.Widget_Ammunition`) true false))

(event `/Game/VRFeature/VirtualRealityBP/Blueprints/PickupActorInterface.Drop`
  (`parent.Drop`)
  (`SceneComponent.SetVisibility` (`self.Widget_Ammunition`) false false))

(event `self.ReceiveBeginPlay`
  (`parent.ReceiveBeginPlay`)
  ;[1 1 1] Obtener referencia
  (bind _aswb_counter (cast `/Game/VRTest/Widgets/WB_Counter` (`WidgetComponent.GetUserWidgetObject` (`self.Widget_Ammunition`))))
  (set `self.Ref_WBCounter` _aswb_counter)
  ;[1 1 1] Actualizar valor inicial
  (`/Game/VRTest/Widgets/WB_Counter.SetValue` (`self.Ref_WBCounter`) (`self.AmmunitionCounter`))
  ;[1 1 1] Ocultar contador
  (`SceneComponent.SetVisibility` (`self.Widget_Ammunition`) false false))

(event `self.CollisionBox_Magazine.OnComponentBeginOverlap`
  (params (OverlappedComponent :type "PrimitiveComponent Object Reference") (OtherActor :type "Actor Object Reference") (OtherComp :type "PrimitiveComponent Object Reference") (OtherBodyIndex :type Integer) (bFromSweep :type Boolean) (SweepResult :type "HitResult Structure (by ref)"))
  (`/Game/VRTest/Blueprints/Base/BP_BaseFunctions_FL.DebugLog` (`KismetStringLibrary.Concat_StrStr` "BeginOverlap with" (`KismetSystemLibrary.GetObjectName` OtherActor)))
  (bind _asbp_pick_up_magazine_a (cast `/Game/VRTest/Blueprints/BP_PickUpMagazine_A` OtherActor))
  (bind _output_get (set `self.Ref_CurrentOverlapMagazine` _asbp_pick_up_magazine_a))
  (add `/Game/VRTest/Blueprints/BP_PickUpMagazine_A.Dropped` _output_get (delegate `OnMagazineDropped`))
  (`/Game/VRTest/Blueprints/BP_MotionController_A.RumbleController` (`self.Ref_CurrentController`) 0.2))

(event `self.CollisionBox_Magazine.OnComponentEndOverlap`
  (params (OverlappedComponent :type "PrimitiveComponent Object Reference") (OtherActor :type "Actor Object Reference") (OtherComp :type "PrimitiveComponent Object Reference") (OtherBodyIndex :type Integer))
  (bind _ref_currentoverlapmagazine (`self.Ref_CurrentOverlapMagazine`))
  (`/Game/VRTest/Blueprints/Base/BP_BaseFunctions_FL.DebugLog` (`KismetStringLibrary.Concat_StrStr` "EndOverlap with" (`KismetSystemLibrary.GetObjectName` OtherActor)))
  (if (== OtherActor _ref_currentoverlapmagazine)
    (remove `/Game/VRTest/Blueprints/BP_PickUpMagazine_A.Dropped` _ref_currentoverlapmagazine (delegate `OnMagazineDropped`))
    (set `self.Ref_CurrentOverlapMagazine` null)))

(event `OnMagazineDropped`
  (remove `/Game/VRTest/Blueprints/BP_PickUpMagazine_A.Dropped` (`self.Ref_CurrentOverlapMagazine`) (delegate `OnMagazineDropped`))
  (`self.LoadMagazine` (`self.Ref_CurrentOverlapMagazine`))
  (set `self.Ref_CurrentOverlapMagazine` null))

(event `self.ReceiveTick`
  (params (DeltaSeconds :type "Float (single-precision)"))
  (`parent.ReceiveTick` DeltaSeconds)
  (`self.ShowLaserTrace`))

(fn `Fire`
  (bind _audio (`self.Audio`))
  (bind _audio_2 (`self.Audio`))
  (bind (_returnvalue_location _returnvalue_rotation) (`KismetMathLibrary.BreakTransform` (`SceneComponent.K2_GetComponentToWorld` (`self.Arrow`))))
  (`KismetSystemLibrary.PrintString` "PickupGun: Fire!")
  (if (> (`self.AmmunitionCounter`) 0)
    ;[1 1 1] Instaciar proyectil
    (`|SpawnActorFromClass` "/Game/VRTest/Blueprints/Weapons/BP_Projectile_A.BP_Projectile_A_C" (`KismetMathLibrary.MakeTransform` _returnvalue_location _returnvalue_rotation (0.25 0.25 0.25)) "Undefined" "OverrideRootScale" null null)
    ;[1 1 1] Hacer temblar el control
    (`/Game/VRTest/Blueprints/BP_MotionController_A.RumbleController` (`self.Ref_CurrentController`) 0.5)
    ;[1 1 1] Reproducir audio
    (`AudioComponent.SetSound` _audio_2 "/Game/VRTest/Sounds/S_GunShot.S_GunShot")
    (`AudioComponent.Play` _audio_2 0.0)
    ;[1 1 1] Actualizar valores
    (`/Engine/EditorBlueprintResources/StandardMacros.DecrementInt` (`self.AmmunitionCounter`)
      (:`  `
        (`self.RefreshAmmoCounter`)))
    (else
      (`KismetSystemLibrary.PrintString` "PickupGun: El arma no tiene municiones")
      ;[1 1 1] Reproducir audio
      (`AudioComponent.SetSound` _audio "/Game/VRTest/Sounds/S_GunEmpty.S_GunEmpty")
      (`AudioComponent.Play` _audio 0.0))))

(fn `LoadMagazine`
  (params (Magazine :type "/Game/VRTest/Blueprints/BP_PickUpMagazine_A Object Reference"))
  (bind _audio (`self.Audio`))
  (`/Game/VRTest/Blueprints/Base/BP_BaseFunctions_FL.DebugLog` "PickUpGun: LoadMagazine")
  (set `self.AmmunitionCounter` (`/Game/VRTest/Blueprints/BP_PickUpMagazine_A.AmmunitionCounter` Magazine))
  (`self.K2_DestroyActor` Magazine)
  (`self.RefreshAmmoCounter`)
  ;[1 1 1] Reproducir audio
  (`AudioComponent.SetSound` _audio "/Game/VRTest/Sounds/S_GunReload.S_GunReload")
  (`AudioComponent.Play` _audio 0.0))

(fn `ShowLaserTrace`
  (bind _arrow (`self.Arrow`))
  (bind _bill_lasertrace (`self.Bill_LaserTrace`))
  (bind _returnvalue (`SceneComponent.K2_GetComponentLocation` _arrow))
  ;[1 1 1] Verificar si hay Hit
  (if (`self.IsPickedUp`)
    (bind (_outhit _returnvalue_2) (`KismetSystemLibrary.LineTraceSingleForObjects` _returnvalue (+ _returnvalue (* (`SceneComponent.GetForwardVector` _arrow) (`self.LaserTraceLength`))) (`|MakeArray` "ObjectTypeQuery2" :!type "EObjectTypeQuery Enum")))
    (if _returnvalue_2
      (cast `/Game/VRTest/Blueprints/Characters/BP_Enemy_A` (`.HitActor` (`GameplayStatics.BreakHitResult` _outhit))
        (:`then`
          ;[1 1 1] Mostrar u ocular la marca laser
          (`SceneComponent.SetVisibility` _bill_lasertrace true false)
          (`SceneComponent.K2_SetRelativeLocation` _bill_lasertrace (`KismetMathLibrary.MakeVector` (- (`.Distance` (`GameplayStatics.BreakHitResult` _outhit)) 10.0)) false false))
        (:`CastFailed`
          (`SceneComponent.SetVisibility` (`self.Bill_LaserTrace`) false false :!label _label)))
      (else
        (goto _label)))
    (else
      (goto _label))))

(fn `UserConstructionScript`
  (`parent.UserConstructionScript`))