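; Throwable-style VR pickup bomb that explodes when its static mesh takes a hard enough hit.
; On component hit, an impulse above MinimalForceToDetonate spawns an explosion emitter, hides the mesh and stops its physics.
; A sphere trace around the bomb then calls Kill on nearby BP_Enemy_A actors, and the bomb destroys itself after a short delay.
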(event `self.StaticMeshComponent.OnComponentHit`
  (params (HitComponent :type "PrimitiveComponent Object Reference") (OtherActor :type "Actor Object Reference") (OtherComp :type "PrimitiveComponent Object Reference") (NormalImpulse :type "Vector Structure") (Hit :type "HitResult Structure (by ref)"))
  (bind _returnvalue (`self.K2_GetActorLocation`))
  (bind _staticmeshcomponent (`self.StaticMeshComponent`))
  (`/Game/VRTest/Blueprints/Base/BP_BaseFunctions_FL.Log` "PickupBomb: Hit")
  ;[1 1 1] Verificar detonación
  (if (> (`KismetMathLibrary.VSize` NormalImpulse) (`self.MinimalForceToDetonate`))
    (`|ExecutionSequence`
      (:`then_0`
        ;[1 1 1] Detonación
        (`GameplayStatics.SpawnEmitterAtLocation` "/Game/StarterContent/Particles/P_Explosion.P_Explosion" (`self.K2_GetActorLocation`))
        (`SceneComponent.SetVisibility` _staticmeshcomponent false false)
        (`PrimitiveComponent.SetSimulatePhysics` _staticmeshcomponent false))
      (:`then_1`
        ;[1 1 1] Afectar enemigos cercanos
        (bind _outhits (`KismetSystemLibrary.SphereTraceMultiForObjects` _returnvalue _returnvalue 100.0 (`|MakeArray` "ObjectTypeQuery2" :!type "EObjectTypeQuery Enum")))
        (for _array_element _outhits
          (bind _asbp_enemy_a (cast `/Game/VRTest/Blueprints/Characters/BP_Enemy_A` (`.HitActor` (`GameplayStatics.BreakHitResult` _array_element))))
          (`/Game/VRTest/Blueprints/Characters/BP_Enemy_A.Kill` _asbp_enemy_a)))
      (:`then_2`
        ;[1 1 1] Eliminar objeto
        (`KismetSystemLibrary.Delay` 0.5)
        (`self.K2_DestroyActor`)))))

(fn `UserConstructionScript`
  (`parent.UserConstructionScript`))