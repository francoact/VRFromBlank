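; BP_RaceController_A runs a timed race by coordinating references to a movable object, a mark collection and a chronometer.
; The object's MoveStarted event resets and starts the chronometer.
; The collection's finish condition stops the clock, then resets the marks and restarts the object's position after a short delay.
; The collection's reset condition performs that same reset immediately, without stopping the clock.
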(event `self.RefMovilObject.MoveStarted`
  (`self.StartRace`))

(event `self.RefMarkCollection.FinishConditionReached`
  (`self.EndRace`)
  (`KismetSystemLibrary.Delay` 5.0)
  (`/Game/VRTest/Blueprints/Mechanisms/BP_MarkCollection_A.ResetCollection` (`self.RefMarkCollection`))
  (`/Game/VRTest/Blueprints/Mechanisms/BP_MovilObject_A.RestartPosition` (`self.RefMovilObject`)))

(event `self.RefMarkCollection.ResetConditionReached`
  (`/Game/VRTest/Blueprints/Mechanisms/BP_MarkCollection_A.ResetCollection` (`self.RefMarkCollection`))
  (`/Game/VRTest/Blueprints/Mechanisms/BP_MovilObject_A.RestartPosition` (`self.RefMovilObject`)))

(fn `EndRace`
  (`/Game/VRTest/Blueprints/Mechanisms/BP_Chronometer_A.Stop` (`self.RefChronometer`)))

(fn `StartRace`
  (`/Game/VRTest/Blueprints/Mechanisms/BP_Chronometer_A.Reset` (`self.RefChronometer`))
  (`/Game/VRTest/Blueprints/Mechanisms/BP_Chronometer_A.Start` (`self.RefChronometer`)))

(fn `UserConstructionScript`)