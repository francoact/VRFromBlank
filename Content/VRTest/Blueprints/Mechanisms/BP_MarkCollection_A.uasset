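; BP_MarkCollection_A is an ordered checkpoint collection, apparently for a maze, where marks must be overlapped in array order.
; The construction script binds each StaticMeshActor's overlap; the current mark hides with a coin sound and advances the index.
; The last mark fires FinishConditionReached with a win sound, while skipping ahead only fires ResetConditionReached.
; ResetCollection, not called internally, restores visibility and progress with a failure sound.
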(event `WinMaseEvent`
  (`self.FinishConditionReached`)
  (`GameplayStatics.PlaySound2D` "/Game/VRTest/Sounds/S_Win_01a.S_Win_01a" 1.0 1.0 0.0 null null))

(fn `OnMarkBeginOverlap`
  (params (ThisActor :type "Actor Object Reference") (OtherActor :type "Actor Object Reference"))
  (bind _asstatic_mesh_actor (cast `StaticMeshActor` ThisActor))
  (`self.OnMarkCheck` (`KismetArrayLibrary.Array_Find` (`self.Marks`) _asstatic_mesh_actor)))

(fn `OnMarkCheck`
  (params (MarkIndex :type Integer :default 0))
  (bind _currentcheck (`self.CurrentCheck`))
  (if (== MarkIndex _currentcheck)
    (`self.ProcessCurrentMark`)
    (elif (> MarkIndex _currentcheck)
      (`self.ResetConditionReached`))))

(fn `ProcessCurrentMark`
  (bind _output (`|GetArrayItem` (`self.Marks`) (`self.CurrentCheck`)))
  (`SceneComponent.SetVisibility` (`StaticMeshActor.StaticMeshComponent` _output) false false)
  (`GameplayStatics.PlaySoundAtLocation` "/Game/VRTest/Sounds/S_Coin.S_Coin" (`self.K2_GetActorLocation` _output) (struct) 3.0 1.0 0.0 null null null)
  (`/Engine/EditorBlueprintResources/StandardMacros.IncrementInt` (`self.CurrentCheck`)
    (:`  `
      ;[1 1 1] Condición de Victoria
      (if (== (`self.CurrentCheck`) (`KismetArrayLibrary.Array_Length` (`self.Marks`)))
        (`self.WinMaseEvent`)))))

(fn `ResetCollection`
  (`GameplayStatics.PlaySound2D` "/Game/VRTest/Sounds/S_Whoops.S_Whoops" 0.2 1.0 0.0 null null)
  (for _array_element (`self.Marks`)
    (`SceneComponent.SetVisibility` (`StaticMeshActor.StaticMeshComponent` _array_element) true false)
    (set `self.CurrentCheck` 0)))

(fn `UserConstructionScript`
  (for _array_element (`self.Marks`)
    (add `self.OnActorBeginOverlap` _array_element (`|CreateDelegate` :!event `OnMarkBeginOverlap`))))