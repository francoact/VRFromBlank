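; VR two-axis lever that an overlapping BP_MotionController_A grips and tilts, snapping back to center on release.
; A zero-delay loop converts hand offset into pitch and roll, using tangent math to clamp tilt within a MaxLeverAngle cone.
; Each update derives a normalized value and axis, calls CallValueUpdated and plays haptics scaled by deflection, throttled to periodic beats near the limit.
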(event `self.SM_Lever.OnComponentBeginOverlap`
  (params (OverlappedComponent :type "PrimitiveComponent Object Reference") (OtherActor :type "Actor Object Reference") (OtherComp :type "PrimitiveComponent Object Reference") (OtherBodyIndex :type Integer) (bFromSweep :type Boolean) (SweepResult :type "HitResult Structure (by ref)"))
  (`/Game/VRTest/Blueprints/Base/BP_BaseFunctions_FL.DebugLog` "Lever: LeverBeginOverlap")
  (bind _asbp_motion_controller_a (cast `/Game/VRTest/Blueprints/BP_MotionController_A` OtherActor))
  (set `self.RefMotionController` _asbp_motion_controller_a)
  (`self.BeginMotionUpdate`))

(event `BeginMotionUpdate`
  (`/Game/VRTest/Blueprints/Base/BP_BaseFunctions_FL.DebugLog` "Lever: BeginMotionUpdate")
  (set `self.UpdateMotion` true)
  (if (`self.UpdateMotion`) :!label _label
    (if (`/Game/VRTest/Blueprints/BP_MotionController_A.bWantsToGrip` (`self.RefMotionController`))
      (set `self.ControllerInitialLocation` (`SceneComponent.K2_GetComponentLocation` (`/Game/VRTest/Blueprints/BP_MotionController_A.MotionController` (`self.RefMotionController`))))
      (set `self.LeverInitialRotation` (`SceneComponent.K2_GetComponentRotation` (`self.SM_Lever`)))
      (`KismetSystemLibrary.Delay` 0.0 :!label _label_2)
      (if (`self.UpdateMotion`)
        (if (`/Game/VRTest/Blueprints/BP_MotionController_A.bWantsToGrip` (`self.RefMotionController`))
          (`self.CalculateClampedRotation`)
          (`SceneComponent.K2_SetWorldRotation` (`self.SM_Lever`) (`self.LeverFinalRotation`) false false)
          (`self.UpdateValues`)
          (goto _label_2)
          (else
            (`|ExecutionSequence`
              (:`then_0`
                _)
              (:`then_1`
                (goto _label))))))
      (`self.RecenterLever`)
      (else
        (`KismetSystemLibrary.Delay` 0.0)
        (goto _label)))
    (else
      (`self.RecenterLever`))))

(event `self.SM_Lever.OnComponentEndOverlap`
  (params (OverlappedComponent :type "PrimitiveComponent Object Reference") (OtherActor :type "Actor Object Reference") (OtherComp :type "PrimitiveComponent Object Reference") (OtherBodyIndex :type Integer))
  (`/Game/VRTest/Blueprints/Base/BP_BaseFunctions_FL.DebugLog` "Lever: LeverEndOverlap")
  (cast `/Game/VRTest/Blueprints/BP_MotionController_A` OtherActor)
  (set `self.RefMotionController` null)
  (`self.EndMotionUpdate`))

(event `EndMotionUpdate`
  (`/Game/VRTest/Blueprints/Base/BP_BaseFunctions_FL.DebugLog` "Lever: EndMotionUpdate")
  (set `self.UpdateMotion` false))

(event `RecenterLever`
  (`/Game/VRTest/Blueprints/Base/BP_BaseFunctions_FL.DebugLog` "Lever: RecenterLever")
  (`SceneComponent.K2_SetWorldRotation` (`self.SM_Lever`) (`KismetMathLibrary.MakeRotator` 0.0) false false))

(fn `CalculateClampedRotation`
  (locals (y :type "Float (double-precision)" :default 0.0) (x :type "Float (double-precision)"))
  (bind (_controllerinitiallocation_x _controllerinitiallocation_y _controllerinitiallocation_z) (`KismetMathLibrary.BreakVector` (`self.ControllerInitialLocation`)))
  (bind (_returnvalue_x _returnvalue_y _returnvalue_z) (`KismetMathLibrary.BreakVector` (`SceneComponent.K2_GetComponentLocation` (`self.SM_Lever`))))
  ;[1 1 1] Sumar desfase a rotación iniciar para obtener nueva
  (bind _output_get (set `self.LeverFinalRotation` (`self.LocToRot` (+ (- (`SceneComponent.K2_GetComponentLocation` (`/Game/VRTest/Blueprints/BP_MotionController_A.MotionController` (`self.RefMotionController`))) (`self.ControllerInitialLocation`)) (`self.RotToLoc` (`self.LeverInitialRotation`) (- _controllerinitiallocation_z _returnvalue_z))))))
  (bind _returnvalue (`KismetMathLibrary.DegTan` (.roll _output_get)))
  (bind _returnvalue_2 (`KismetMathLibrary.DegTan` (.pitch _output_get)))
  (bind _returnvalue_3 (`KismetMathLibrary.FClamp` (`KismetMathLibrary.Sqrt` (+ (`KismetMathLibrary.Square` _returnvalue) (`KismetMathLibrary.Square` _returnvalue_2))) 0.0 (`KismetMathLibrary.DegTan` (`self.MaxLeverAngle`))))
  ;[1 1 1] Restringir rotaciones
  (set `self.LeverFinalAngle` (`KismetMathLibrary.DegAtan` _returnvalue_3))
  (bind _returnvalue_4 (/ _returnvalue _returnvalue_2))
  (bind _output_get_2 (set `local.y` (* (/ _returnvalue_3 (`KismetMathLibrary.Sqrt` (+ 1.0 (`KismetMathLibrary.Square` _returnvalue_4)))) (select `bool` (< _returnvalue_2 0.0) :`false` 1.0 :`true` -1.0 :!type "Float (single-precision)")))) ; Y
  (set `self.LeverFinalRotation` (`KismetMathLibrary.MakeRotator` (`KismetMathLibrary.DegAtan2` (* _output_get_2 _returnvalue_4) 1.0) (`KismetMathLibrary.DegAtan2` _output_get_2 1.0)))
  (return))

(fn `PlayHapticEffect`
  (bind _returnvalue (`GameplayStatics.GetTimeSeconds`))
  (`/Engine/EditorBlueprintResources/StandardMacros.IsValid` (`self.RefMotionController`)
    (:`Is Valid`
      (if (< (`self.NormalizedValue`) 0.99)
        (`PlayerController.PlayHapticEffect` (`GameplayStatics.GetPlayerController` 0) "/Game/VRFeature/VirtualRealityBP/Blueprints/NewHapticFeedbackEffect_Curve.NewHapticFeedbackEffect_Curve" (`/Game/VRTest/Blueprints/BP_MotionController_A.Hand` (`self.RefMotionController`)) (* (`self.NormalizedValue`) 0.3) false :!label _label)
        (elif (> (- _returnvalue (`self.LastHapticBeat`)) 0.5)
          (`|ExecutionSequence`
            (:`then_0`
              (goto _label))
            (:`then_1`
              (set `self.LastHapticBeat` _returnvalue))))))))

(fn `UpdateValues`
  (locals (MaxValue :type "Float (double-precision)" :default 0.0))
  (bind (_leverfinalrotation_roll _leverfinalrotation_pitch) (`KismetMathLibrary.BreakRotator` (`self.LeverFinalRotation`)))
  (bind _maxleverangle (`self.MaxLeverAngle`))
  (set `self.NormalizedValue` (/ (`self.LeverFinalAngle`) (`self.MaxLeverAngle`)))
  (set `self.NormalizedAxis` (`KismetMathLibrary.MakeVector2D` (- 0.0 (/ _leverfinalrotation_pitch _maxleverangle)) (/ _leverfinalrotation_roll _maxleverangle)))
  (`|ExecutionSequence`
    (:`then_1`
      (`self.ValueUpdated`))
    (:`then_2`
      (`self.PlayHapticEffect`))))

(fn `UserConstructionScript`)