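; VR keyhole mechanism that accepts a BP_PickUp_Key_A with a matching KeyValue, snapping it to AttachPoint and disabling pickup.
; With a key inserted, a gripping controller's roll turns the Pivot within a clamped quarter turn, polled by a zero-Delay loop.
; Full turn locks it and calls KeyLocked, otherwise it unlocks, with State coloring a text indicator.
; ControllerIn/Out logic is disconnected, and IsLock tests a state never set here.
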(event `self.Col_Key.OnComponentBeginOverlap`
  (params (OverlappedComponent :type "PrimitiveComponent Object Reference") (OtherActor :type "Actor Object Reference") (OtherComp :type "PrimitiveComponent Object Reference") (OtherBodyIndex :type Integer) (bFromSweep :type Boolean) (SweepResult :type "HitResult Structure (by ref)"))
  (`/Game/VRTest/Blueprints/Base/BP_BaseFunctions_FL.DebugLog` "KeyHolder: BeginOverlap")
  (bind _asbp_pick_up_key_a (cast `/Game/VRTest/Blueprints/Mechanisms/BP_PickUp_Key_A` OtherActor))
  (if (`KismetStringLibrary.EqualEqual_StrStr` (`/Game/VRTest/Blueprints/Mechanisms/BP_PickUp_Key_A.KeyValue` _asbp_pick_up_key_a) (`self.KeyValue`))
    ;[1 1 1] Ingresar llave
    (`/Game/VRTest/Blueprints/BP_PickUpStaticMesh_A.Drop` _asbp_pick_up_key_a)
    (`PrimitiveComponent.SetSimulatePhysics` (`StaticMeshActor.StaticMeshComponent` _asbp_pick_up_key_a) false)
    (`self.K2_AttachToComponent` _asbp_pick_up_key_a (`self.AttachPoint`) "None" "SnapToTarget" "SnapToTarget" "KeepWorld" false)
    (set `/Game/VRTest/Blueprints/BP_PickUpStaticMesh_A.CanPickUp` false _asbp_pick_up_key_a) ; Desactivar PickUp
    (`self.KeyOn`)))

(event `self.Col_Controller.OnComponentBeginOverlap`
  (params (OverlappedComponent :type "PrimitiveComponent Object Reference") (OtherActor :type "Actor Object Reference") (OtherComp :type "PrimitiveComponent Object Reference") (OtherBodyIndex :type Integer) (bFromSweep :type Boolean) (SweepResult :type "HitResult Structure (by ref)"))
  (bind _asbp_motion_controller_a (cast `/Game/VRTest/Blueprints/BP_MotionController_A` OtherActor))
  (set `self.MotionController` _asbp_motion_controller_a)
  (`self.ControllerIn`)
  (`self.BeginRotationUpdate`))

(event `self.Col_Controller.OnComponentEndOverlap`
  (params (OverlappedComponent :type "PrimitiveComponent Object Reference") (OtherActor :type "Actor Object Reference") (OtherComp :type "PrimitiveComponent Object Reference") (OtherBodyIndex :type Integer))
  (cast `/Game/VRTest/Blueprints/BP_MotionController_A` OtherActor)
  (set `self.MotionController` null)
  (`self.ControllerOut`)
  (`self.EndRotationUpdate`))

(event `BeginRotationUpdate`
  (bind _relativerotation_roll (`KismetMathLibrary.BreakRotator` (`SceneComponent.RelativeRotation` (`self.Pivot`))))
  (bind _relativerotation_roll_2 (`KismetMathLibrary.BreakRotator` (`SceneComponent.RelativeRotation` (`/Game/VRTest/Blueprints/BP_MotionController_A.MotionController` (`self.MotionController`)))))
  (bind _relativerotation_roll_3 (`KismetMathLibrary.BreakRotator` (`SceneComponent.RelativeRotation` (`/Game/VRTest/Blueprints/BP_MotionController_A.MotionController` (`self.MotionController`)))))
  (bind _returnvalue (- _relativerotation_roll_2 (`self.MotionControllerInitialRotation`)))
  (bind _returnvalue_2 (`KismetMathLibrary.FClamp` (- (`self.KeyHolderInitialRotation`) (select `bool` (< (`KismetMathLibrary.Abs` _returnvalue) 3.0) :`false` _returnvalue)) -90.0 0.0))
  (set `self.IsMotionController` true)
  (if (`self.IsMotionController`) :!label _label
    (if (> (`self.State`) 0)
      (if (`/Game/VRTest/Blueprints/BP_MotionController_A.bWantsToGrip` (`self.MotionController`))
        (set `self.MotionControllerInitialRotation` _relativerotation_roll_3)
        (set `self.KeyHolderInitialRotation` _relativerotation_roll)
        ;[1 1 1] Actualizar Rotación (por frame)
        (`SceneComponent.K2_SetRelativeRotation` (`self.Pivot`) (`KismetMathLibrary.MakeRotator` _returnvalue_2) false false :!label _label_2)
        (if (`KismetMathLibrary.NearlyEqual_FloatFloat` _returnvalue_2 -90.0)
          (`self.LockIn`)
          (else
            (`self.LockOut`)))
        (`KismetSystemLibrary.Delay` 0.0)
        (if (`self.IsMotionController`)
          (if (`/Game/VRTest/Blueprints/BP_MotionController_A.bWantsToGrip` (`self.MotionController`))
            (goto _label_2)
            (else
              (goto _label))))
        (else
          (`KismetSystemLibrary.Delay` 0.0 :!label _label_3)
          (goto _label)))
      (else
        (goto _label_3)))))

(event `EndRotationUpdate`
  (set `self.IsMotionController` false))

(fn `ControllerIn`)

(fn `ControllerOut`)

(fn `IsLock`
  (returns (ReturnValue :type Boolean))
  (return (== (`self.State`) 4)))

(fn `KeyOn`
  (set `self.State` 1)
  (`self.UpdateUI_State`))

(fn `LockIn`
  (set `self.State` 3)
  (`self.UpdateUI_State`)
  (`self.KeyLocked`))

(fn `LockOut`
  (set `self.State` 1)
  (`self.UpdateUI_State`))

(fn `UserConstructionScript`)