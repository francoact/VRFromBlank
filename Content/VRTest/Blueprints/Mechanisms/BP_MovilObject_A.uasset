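; BP_MovilObject_A is a movable mechanism actor, in a VR test project, that a referenced lever drives.
; Each RefLever ValueUpdated event adds a swept local offset from the lever's normalized 2D axis, scaled by LeverSpeedScale, with zero Z.
; Movement advances per lever update, without delta-time scaling.
; BeginPlay stores the start location, and RestartPosition moves the actor back to it without sweeping.
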(event `self.ReceiveBeginPlay`
  (set `self.StartPosition` (`self.K2_GetActorLocation`)))

(event `self.ReceiveTick`
  (params (DeltaSeconds :type "Float (single-precision)")))

(event `self.RefLever.ValueUpdated`
  (`self.K2_AddActorLocalOffset` (* (`KismetMathLibrary.Conv_Vector2DToVector` (`/Game/VRTest/Blueprints/Mechanisms/BP_Lever_A.NormalizedAxis` (`self.RefLever`))) (`self.LeverSpeedScale`)) true))

(fn `RestartPosition`
  (`self.K2_SetActorLocation` (`self.StartPosition`)))

(fn `UserConstructionScript`)