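; BP_Chronometer_A is a chronometer actor that shows elapsed time on a text render component.
; Tick writes Time as zero-padded minutes, seconds and sixtieths of a second, then adds delta seconds.
; Reset zeroes Time and Start enables actor tick.
; Stop also enables tick instead of disabling it, so it does not pause the count.
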(event `self.ReceiveTick`
  (params (DeltaSeconds :type "Float (single-precision)"))
  (bind _time (`self.Time`))
  (bind _returnvalue (`KismetMathLibrary.FTrunc` _time))
  (bind _returnvalue_2 (mod _returnvalue 60))
  (bind _returnvalue_3 (/ _returnvalue 60))
  (bind _returnvalue_4 (`KismetMathLibrary.FTrunc` (* (`KismetMathLibrary.Fraction` _time) 60.0)))
  (`TextRenderComponent.K2_SetText` (`self.TextRender`) (`KismetTextLibrary.Conv_StringToText` (`KismetStringLibrary.Concat_StrStr` (select `bool` (< _returnvalue_3 10) :`true` "0") (`KismetStringLibrary.Conv_IntToString` _returnvalue_3) ":" (select `bool` (< _returnvalue_2 10) :`true` "0") (`KismetStringLibrary.Conv_IntToString` _returnvalue_2) ":" (select `bool` (< _returnvalue_4 10) :`true` "0") (`KismetStringLibrary.Conv_IntToString` _returnvalue_4))))
  (set `self.Time` (+ (`self.Time`) DeltaSeconds)))

(fn `Reset`
  (set `self.Time` 0.0))

(fn `Start`
  (`self.SetActorTickEnabled` true))

(fn `Stop`
  (`self.SetActorTickEnabled` true))

(fn `UserConstructionScript`)